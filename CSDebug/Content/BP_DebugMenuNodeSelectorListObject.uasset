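; Data object for one entry in a debug menu node selector list, controlling that entry's selection highlight.
; OnSelect and OnNoSelect show or hide a translucent orange tint on the background border of its node widget, when that widget is valid.
; CheckSelect reapplies the highlight when the list widget's selected index matches its own, working around selection not being set properly at initialization.
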(fn OnSelect
  (bind _mlistnodewidget (Variables|Default|GetmListNodeWidget))
  (if (Utilities|IsValid _mlistnodewidget)
    (Class|Border|SetBrushColor (Variables|/CSDebug/WB_DebugMenuNodeSelectorListItem.WB_DebugMenuNodeSelectorListItem_C|GetBorder_BackGround _mlistnodewidget) "(R=1.000000,G=0.568627,B=0.000000,A=0.298039)")))

(fn OnNoSelect
  (bind _mlistnodewidget (Variables|Default|GetmListNodeWidget))
  (if (Utilities|IsValid _mlistnodewidget)
    (Class|Border|SetBrushColor (Variables|/CSDebug/WB_DebugMenuNodeSelectorListItem.WB_DebugMenuNodeSelectorListItem_C|GetBorder_BackGround _mlistnodewidget) "(R=1.000000,G=0.568627,B=0.000000,A=0.000000)")))

(fn CheckSelect
  (if (== (Variables|/CSDebug/WB_DebugMenuNodeSelector.WB_DebugMenuNodeSelector_C|GetmSelectIndex (Variables|Default|GetmListWidget)) (Variables|Default|GetmIndex))
    (CallFunction|OnSelect)))