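; Data object for a row in the debug menu list view, driving the look of its WB_DebugMenuListItem widget.
; SetViewNode binds the row widget, then triggers select or deselect by comparing its list index to the menu's selected index.
; Selection tints the row background translucent orange and deselection clears it.
; Decide and value-name events refresh the row's value text from GetValueName.
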(event EventOnSelectBP
  (bind _returnvalue (Class|CSDebugMenuListObjectBase|GetDebugMenuWidgetNode))
  (bind (_aswb_debug_menu_list_item _bsuccess) (Utilities|Casting|CastToWB_DebugMenuListItem _returnvalue))
  (if _bsuccess
    (Class|Border|SetBrushColor (Variables|/CSDebug/WB_DebugMenuListItem.WB_DebugMenuListItem_C|GetBorder_BackGround _aswb_debug_menu_list_item) "(R=1.000000,G=0.569874,B=0.000000,A=0.300000)")))

(event EventOnNoSelectBP
  (bind _returnvalue (Class|CSDebugMenuListObjectBase|GetDebugMenuWidgetNode))
  (bind (_aswb_debug_menu_list_item _bsuccess) (Utilities|Casting|CastToWB_DebugMenuListItem _returnvalue))
  (if _bsuccess
    (Class|Border|SetBrushColor (Variables|/CSDebug/WB_DebugMenuListItem.WB_DebugMenuListItem_C|GetBorder_BackGround _aswb_debug_menu_list_item) "(R=0.000000,G=0.000000,B=0.000000,A=0.000000)")))

(event EventOnDecideBP
  (CallFunction|SetValueNameWidget))

(event EventOnSetValueNameBP
  (CallFunction|SetValueNameWidget))

(fn SetViewNode
  (params (InNode :type WB%20Debug%20Menu%20List%20Item%20Object%20Reference))
  (Class|CSDebugMenuListObjectBase|SetDebugMenuWidgetNode InNode)
  (if (== (Class|CSDebugMenuListObjectBase|GetListViewIndex) (Class|CSDebugMenuWidgetBase|GetSelectIndex (.AsWB%20Debug%20Menu (Utilities|Casting|CastToWB_DebugMenu (Class|CSDebugMenuListObjectBase|GetDebugMenuWidget)))))
    (Class|CSDebugMenuListObjectBase|OnSelect)
    (else
      (Class|CSDebugMenuListObjectBase|OnNoSelect))))

(fn SetValueNameWidget
  (bind _returnvalue (Class|CSDebugMenuListObjectBase|GetDebugMenuWidgetNode))
  (bind (_aswb_debug_menu_list_item _bsuccess) (Utilities|Casting|CastToWB_DebugMenuListItem _returnvalue))
  (if _bsuccess
    (Rendering|Components|TextRender|SetText (Variables|/CSDebug/WB_DebugMenuListItem.WB_DebugMenuListItem_C|GetTextBlock_Value _aswb_debug_menu_list_item) (Utilities|Text|ToText(String) (Class|CSDebugMenuListObjectBase|GetValueName)))))